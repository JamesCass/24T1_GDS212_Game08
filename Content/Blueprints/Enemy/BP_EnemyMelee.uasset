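; Melee enemy pawn drawn with flipbook sprites that chases and attacks the first-person player.
; Pawn sensing or an ArenaMode event starts AI MoveTo; on arrival it stops, plays the attack, damages the player, then re-enables movement.
; Once it has a target, Tick yaws it toward the player.
; Each hit shows a HUD hitmarker and costs one health, causing a brief stagger or a death animation, corpse and delayed destruction.
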(event `ArenaMode`
  (bind _enemyflipbook (`self.EnemyFlipbook`))
  (bind _asbp_first_person_character (cast `/Game/FirstPerson/Blueprints/BP_FirstPersonCharacter` (`self.PlayerRef`)))
  (set `self.CanSeePlayer?` true)
  (`|AIMoveTo` self (0.0 0.0 0.0) _asbp_first_person_character
    (:`OnSuccess`
      (`/Engine/EditorBlueprintResources/StandardMacros.DoOnce` false :!label _label
        (:`Completed`
          (if (not (`self.IsDead?`))
            (`ActorComponent.Deactivate` (`self.CharacterMovement`))
            (`PaperFlipbookComponent.SetFlipbook` _enemyflipbook "/Game/Sprites/Enemies/Melee/FB_MeleeAttack.FB_MeleeAttack")
            (`self.AttackPlayer`)
            (`KismetSystemLibrary.Delay` (`PaperFlipbookComponent.GetFlipbookLength` _enemyflipbook))
            (`PaperFlipbookComponent.SetFlipbook` (`self.EnemyFlipbook`) "/Game/Sprites/Enemies/Melee/FB_MeeleMove.FB_MeeleMove")
            (`ActorComponent.Activate` (`self.CharacterMovement`) false)
            (goto _label :!via `Reset`)))))))

(event `self.ReceiveBeginPlay`
  (bind _returnvalue (`GameplayStatics.GetActorOfClass` "/Game/FirstPerson/Blueprints/BP_FirstPersonCharacter.BP_FirstPersonCharacter_C"))
  (set `self.PlayerRef` _returnvalue))

(event `self.ReceiveTick`
  (params (DeltaSeconds :type "Float (single-precision)"))
  (bind (_returnvalue_roll _returnvalue_pitch _returnvalue_yaw) (`KismetMathLibrary.BreakRotator` (`KismetMathLibrary.FindLookAtRotation` (`self.K2_GetActorLocation`) (`self.K2_GetActorLocation` (`GameplayStatics.GetPlayerCharacter` 0)))))
  (if (`self.CanSeePlayer?`)
    (`self.K2_SetActorRotation` (`KismetMathLibrary.MakeRotator` 0.0 0.0 _returnvalue_yaw))))

(event `self.PawnSensing.OnSeePawn`
  (params (Pawn :type "Pawn Object Reference"))
  (bind _enemyflipbook (`self.EnemyFlipbook`))
  (bind _asbp_first_person_character (cast `/Game/FirstPerson/Blueprints/BP_FirstPersonCharacter` Pawn))
  (set `self.CanSeePlayer?` true)
  (`|AIMoveTo` self (0.0 0.0 0.0) _asbp_first_person_character
    (:`OnSuccess`
      (`/Engine/EditorBlueprintResources/StandardMacros.DoOnce` false :!label _label_2
        (:`Completed`
          (if (not (`self.IsDead?`))
            (`ActorComponent.Deactivate` (`self.CharacterMovement`))
            (`PaperFlipbookComponent.SetFlipbook` _enemyflipbook "/Game/Sprites/Enemies/Melee/FB_MeleeAttack.FB_MeleeAttack")
            (`self.AttackPlayer`)
            (`KismetSystemLibrary.Delay` (`PaperFlipbookComponent.GetFlipbookLength` _enemyflipbook))
            (`PaperFlipbookComponent.SetFlipbook` (`self.EnemyFlipbook`) "/Game/Sprites/Enemies/Melee/FB_MeeleMove.FB_MeeleMove")
            (`ActorComponent.Activate` (`self.CharacterMovement`) false)
            (goto _label_2 :!via `Reset`)))))))

(event `self.ReceiveAnyDamage`
  (params (Damage :type "Float (single-precision)") (DamageType :type "DamageType Object Reference") (InstigatedBy :type "Controller Object Reference") (DamageCauser :type "Actor Object Reference"))
  (bind _foundwidgets (`WidgetBlueprintLibrary.GetAllWidgetsOfClass` "/Game/Blueprints/UI/BP_HUD.BP_HUD_C"))
  (`/Game/Blueprints/UI/BP_HUD.Hitmarker` _foundwidgets)
  (set `self.TotalHealth` (- (`self.TotalHealth`) 1))
  (if (<= (`self.TotalHealth`) 0)
    (`self.KillMeleeEnemy`)
    (else
      (`self.DamageMeleeEnemy`))))

(event `KillMeleeEnemy`
  (bind _enemyflipbook (`self.EnemyFlipbook`))
  (`/Engine/EditorBlueprintResources/StandardMacros.DoOnce` false
    (:`Completed`
      (set `self.IsDead?` true)
      (`ActorComponent.Deactivate` (`self.CharacterMovement`))
      (`PrimitiveComponent.SetCollisionEnabled` (`self.CapsuleComponent`) "NoCollision")
      (`PaperFlipbookComponent.SetFlipbook` _enemyflipbook "/Game/Sprites/Enemies/Melee/FB_MeleeDeath.FB_MeleeDeath")
      (`KismetSystemLibrary.Delay` (`PaperFlipbookComponent.GetFlipbookLength` _enemyflipbook))
      (`PaperFlipbookComponent.SetFlipbook` (`self.EnemyFlipbook`) "/Game/Sprites/Enemies/Melee/FB_MeleeDeadBody.FB_MeleeDeadBody")
      (`KismetSystemLibrary.Delay` 4.0)
      (`self.K2_DestroyActor`))))

(event `DamageMeleeEnemy`
  (`PaperFlipbookComponent.SetFlipbook` (`self.EnemyFlipbook`) "/Game/Sprites/Enemies/Melee/FB_MeleeTakeDamage.FB_MeleeTakeDamage")
  (`ActorComponent.Deactivate` (`self.CharacterMovement`))
  (`KismetSystemLibrary.Delay` 0.2)
  (`PaperFlipbookComponent.SetFlipbook` (`self.EnemyFlipbook`) "/Game/Sprites/Enemies/Melee/FB_MeeleMove.FB_MeeleMove")
  (`ActorComponent.Activate` (`self.CharacterMovement`) false))

(event `AttackPlayer`
  (bind _asbp_first_person_character (cast `/Game/FirstPerson/Blueprints/BP_FirstPersonCharacter` (`self.PlayerRef`)))
  (`/Game/FirstPerson/Blueprints/BP_FirstPersonCharacter.TakeMeleeDamage` _asbp_first_person_character))

(fn `UserConstructionScript`)