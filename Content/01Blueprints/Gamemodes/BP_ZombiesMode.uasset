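; Zombie wave game mode that runs successive waves up to a maximum, where the win is only a debug print.
; BeginPlay spawns the first wave, then creates the HUD and sets game-only input.
; Each wave's zombie count scales with the wave number, split between two spawn locations.
; ZombieKilled counts down the remainder, and at zero the next wave spawns after a HUD announcement and short delay.
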(event `WaveStart`
  (`/Game/01Blueprints/UI/BP_ZombiesHUD.ShowWaveStarting` (`self.ZombiesHUDRef`))
  (`KismetSystemLibrary.Delay` 5.0)
  (`self.SpawnZombies`))

(event `self.ReceiveBeginPlay`
  (`self.StartGame`)
  (bind _returnvalue (`|CreateWidget` "/Game/01Blueprints/UI/BP_ZombiesHUD.BP_ZombiesHUD_C"))
  (bind _output_get (set `self.ZombiesHUDRef` _returnvalue))
  (`UserWidget.AddToViewport` _output_get 0)
  (`WidgetBlueprintLibrary.SetInputMode_GameOnly` (`GameplayStatics.GetPlayerController` 0)))

(event `StartGame`
  (`self.SpawnZombies`))

(event `SpawnZombies`
  (bind _output_get (set `self.ZombieTotal` (* (`self.CurrentWave`) 4)))
  (set `self.ZombiesLeft` _output_get)
  (for _index (range (+ _output_get 1))
    (if (== _index (/ (`self.ZombieTotal`) 2))
      (break)
      (else
        (`|SpawnActorFromClass` "/Game/01Blueprints/Enemy/BP_Zombie.BP_Zombie_C" (`self.SpawnLocation1`) "Undefined" "MultiplyWithRoot" null null)
        (`KismetSystemLibrary.PrintString` "spawn1"))))
  (for _ (range 1 (+ (/ (`self.ZombieTotal`) 2) 1))
    (`|SpawnActorFromClass` "/Game/01Blueprints/Enemy/BP_Zombie.BP_Zombie_C" (`self.SpawnLocation2`) "Undefined" "MultiplyWithRoot" null null)
    (`KismetSystemLibrary.PrintString` "spawn2")))

(event `ZombieKilled`
  (bind _result (`/Engine/EditorBlueprintResources/StandardMacros.DecrementInt` (`self.ZombiesLeft`))
    (:`  `
      (if (== _result 0)
        (`self.WaveIncrement`)))))

(event `WaveIncrement`
  (if (== (`self.CurrentWave`) (`self.MaxWaves`))
    (`KismetSystemLibrary.PrintString` "PlayerWinsGame")
    (else
      (`/Engine/EditorBlueprintResources/StandardMacros.IncrementInt` (`self.CurrentWave`)
        (:`  `
          (`self.WaveStart`))))))

(fn `UserConstructionScript`)