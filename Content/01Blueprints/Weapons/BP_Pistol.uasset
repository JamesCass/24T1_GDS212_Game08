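; Pistol weapon Blueprint that fires with limited ammo and animates as a Paper2D flipbook.
; ShootWeapon checks ammo behind a DoOnce gate, spends a round, calls FireWeapon and triggers Flash on the first-person character.
; It then plays the shoot flipbook, waits for its length, returns to idle and reopens the gate through ResetWeapon, so the animation sets the fire rate.
; AddPistolAmmo adds a small fixed amount of ammo.
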(event `self.ShootWeapon`
  (bind _weaponflipbook (`self.WeaponFlipbook`))
  ;[0 0 0] When called call fire weapon raycast, trigger muzzle flash then play pistol firing flipbook then reset.
  (if (> (`self.PistolAmmo`) 0)
    (`/Engine/EditorBlueprintResources/StandardMacros.DoOnce` false :!label _label
      (:`Completed`
        (set `self.PistolAmmo` (- (`self.PistolAmmo`) 1))
        (`self.FireWeapon`)
        (bind _returnvalue (`GameplayStatics.GetActorOfClass` "/Game/01Blueprints/BP_FirstPersonCharacter.BP_FirstPersonCharacter_C"))
        (`/Game/01Blueprints/BP_FirstPersonCharacter.Flash` _returnvalue)
        (`PaperFlipbookComponent.SetFlipbook` _weaponflipbook "/Game/04Assets/Packs/Sprites/Weapons/Pistol/FB_PistolShoot.FB_PistolShoot")
        (`KismetSystemLibrary.Delay` (`PaperFlipbookComponent.GetFlipbookLength` _weaponflipbook))
        (`PaperFlipbookComponent.SetFlipbook` (`self.WeaponFlipbook`) "/Game/04Assets/Packs/Sprites/Weapons/Pistol/FB_PistolIdle.FB_PistolIdle")
        (`self.ResetWeapon`)))))

(event `ResetWeapon`
  ;[0 0 0] When called call fire weapon raycast, trigger muzzle flash then play pistol firing flipbook then reset.
  (goto _label :!via `Reset`))

(event `AddPistolAmmo`
  ;[0 0 0] When called increase ammo count +2
  (set `self.PistolAmmo` (+ (`self.PistolAmmo`) 2)))

(fn `UserConstructionScript`
  (`parent.UserConstructionScript`))