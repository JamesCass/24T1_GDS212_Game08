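; BP_Shotgun is a sprite-based shotgun weapon for the first-person character, firing while shells remain.
; A DoOnce gates each shot, which spends a shell, calls FireWeapon, flashes the player, plays sounds and shows the shoot flipbook, then resets once the animation length elapses.
; AddShotgunAmmo grants shells, and WeaponBobbing plays a bob sequence while moving, otherwise stopping it and easing the flipbook toward zero offset.
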(event `self.ShootWeapon`
  (bind _weaponflipbook (`self.WeaponFlipbook`))
  (if (> (`self.ShotGunAmmo`) 0)
    (`/Engine/EditorBlueprintResources/StandardMacros.DoOnce` false :!label _label
      (:`Completed`
        (set `self.ShotGunAmmo` (- (`self.ShotGunAmmo`) 1))
        (`self.FireWeapon`)
        (bind _returnvalue (`GameplayStatics.GetActorOfClass` "/Game/01Blueprints/BP_FirstPersonCharacter.BP_FirstPersonCharacter_C"))
        (`/Game/01Blueprints/BP_FirstPersonCharacter.Flash` _returnvalue)
        (`GameplayStatics.PlaySound2D` "/Game/04Assets/Audio/Guns/Shotgun/dsdshtgn.dsdshtgn" 1.0 1.0 0.0 null null)
        (`PaperFlipbookComponent.SetFlipbook` _weaponflipbook "/Game/04Assets/Packs/Sprites/Weapons/Shotgun/FB_ShotgunShoot.FB_ShotgunShoot")
        (`GameplayStatics.PlaySound2D` "/Game/04Assets/Audio/Guns/Shotgun/old-school-shotgun-reload.old-school-shotgun-reload" 1.0 1.0 0.0 null null)
        (`KismetSystemLibrary.Delay` (`PaperFlipbookComponent.GetFlipbookLength` _weaponflipbook))
        (`PaperFlipbookComponent.SetFlipbook` (`self.WeaponFlipbook`) "/Game/04Assets/Packs/Sprites/Weapons/Shotgun/FB_ShotgunIdle.FB_ShotgunIdle")
        (`self.ResetWeapon`)))))

(event `ResetWeapon`
  (goto _label :!via `Reset`))

(event `AddShotgunAmmo`
  (set `self.ShotGunAmmo` (+ (`self.ShotGunAmmo`) 2)))

(event `WeaponBobbing`
  (params (`IsMoving?` :type Boolean) (DeltaSeconds :type "Float (double-precision)"))
  (bind _weaponflipbook (`self.WeaponFlipbook`))
  (bind _sequenceplayer (`ActorSequenceComponent.SequencePlayer` (`self.WeaponBob`)))
  (if `IsMoving?`
    (`MovieSceneSequencePlayer.Play` _sequenceplayer)
    (else
      (`MovieSceneSequencePlayer.Stop` _sequenceplayer)
      (`SceneComponent.K2_SetRelativeLocation` _weaponflipbook (`KismetMathLibrary.VInterpTo` (`SceneComponent.RelativeLocation` _weaponflipbook) (0.0 0.0 0.0) DeltaSeconds 1.0) false false))))

(fn `UserConstructionScript`
  (`parent.UserConstructionScript`))