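; Melee zombie enemy drawn as a flipbook sprite that yaws to face the player.
; From BeginPlay it chases the player via AIMoveTo and loops timed attacks calling TakeMeleeDamage; ArenaMode offers a similar chase, and pawn sensing is empty.
; Any damage flashes the HUD hitmarker and removes one health, with a DoOnce-gated stun.
; Death plays animations, drops pistol ammo, notifies BP_ZombiesMode and destroys the actor after a delay.
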(event `self.ReceiveTick`
  (params (DeltaSeconds :type "Float (single-precision)"))
  (bind (_returnvalue_roll _returnvalue_pitch _returnvalue_yaw) (`KismetMathLibrary.BreakRotator` (`KismetMathLibrary.FindLookAtRotation` (`self.K2_GetActorLocation`) (`self.K2_GetActorLocation` (`GameplayStatics.GetPlayerCharacter` 0)))))
  ;[0 0 0] Billboard towards player
  (if (`self.CanSeePlayer?`)
    (`self.K2_SetActorRotation` (`KismetMathLibrary.MakeRotator` 0.0 0.0 _returnvalue_yaw))))

(event `ArenaMode`
  (bind _enemyflipbook (`self.EnemyFlipbook`))
  ;[0 0 0] When arena mode activated direclty move towards player
  (bind _asbp_first_person_character (cast `/Game/01Blueprints/BP_FirstPersonCharacter` (`self.PlayerRef`)))
  (set `self.CanSeePlayer?` true)
  (`|AIMoveTo` self (0.0 0.0 0.0) _asbp_first_person_character
    (:`OnSuccess`
      (`/Engine/EditorBlueprintResources/StandardMacros.DoOnce` false :!label _label
        (:`Completed`
          (if (not (`self.IsDead?`))
            (`ActorComponent.Deactivate` (`self.CharacterMovement`))
            (`PaperFlipbookComponent.SetFlipbook` _enemyflipbook "/Game/04Assets/Packs/Sprites/Enemies/Zombie/FB_ZombieAttack.FB_ZombieAttack")
            (`self.AttackPlayer`)
            (`KismetSystemLibrary.Delay` (`PaperFlipbookComponent.GetFlipbookLength` _enemyflipbook))
            (`PaperFlipbookComponent.SetFlipbook` (`self.EnemyFlipbook`) "/Game/04Assets/Packs/Sprites/Enemies/Zombie/FB_ZombieWalk.FB_ZombieWalk")
            (`ActorComponent.Activate` (`self.CharacterMovement`) false)
            (goto _label :!via `Reset`)))))))

(event `self.ReceiveAnyDamage`
  (params (Damage :type "Float (single-precision)") (DamageType :type "DamageType Object Reference") (InstigatedBy :type "Controller Object Reference") (DamageCauser :type "Actor Object Reference"))
  ;[0 0 0] On take damage toggle hitmarker and remove health, if health 0 or below call kill enemy or take damage
  (bind _foundwidgets (`WidgetBlueprintLibrary.GetAllWidgetsOfClass` "/Game/01Blueprints/UI/BP_HUD.BP_HUD_C"))
  (`/Game/01Blueprints/UI/BP_HUD.Hitmarker` _foundwidgets)
  (set `self.TotalHealth` (- (`self.TotalHealth`) 1))
  (if (< (`self.TotalHealth`) 0)
    (`/Engine/EditorBlueprintResources/StandardMacros.DoOnce` false
      (:`Completed`
        (`self.KillMeleeEnemy`)
        (`KismetSystemLibrary.PrintString` "KillMeleeEnemy")))
    (else
      (`/Engine/EditorBlueprintResources/StandardMacros.DoOnce` false
        (:`Completed`
          (`self.DamageMeleeEnemy`)
          (`KismetSystemLibrary.PrintString` "Damage taken"))))))

(event `MoveToPlayerAgain`
  (bind _enemyflipbook (`self.EnemyFlipbook`))
  ;[0 0 0] When see player move towards
  (`|AIMoveTo` self (0.0 0.0 0.0) (stale _asbp_first_person_character) 15.0 :!label _label_2
    (:`OnSuccess`
      (`KismetSystemLibrary.PrintString` "moving towards player")
      ;[0 0 0] When at player play attack animation and call take player damager
      (`/Engine/EditorBlueprintResources/StandardMacros.DoOnce` false :!label _label_3
        (:`Completed`
          (if (not (`self.IsDead?`))
            (`ActorComponent.Deactivate` (`self.CharacterMovement`))
            (`GameplayStatics.PlaySound2D` "/Game/04Assets/Audio/Zombie/zombieAttack.zombieAttack" 1.0 1.0 0.0 null null)
            (`PaperFlipbookComponent.SetFlipbook` _enemyflipbook "/Game/04Assets/Packs/Sprites/Enemies/Zombie/FB_ZombieAttack.FB_ZombieAttack")
            (`self.AttackPlayer`)
            (`KismetSystemLibrary.Delay` (`PaperFlipbookComponent.GetFlipbookLength` _enemyflipbook))
            (`PaperFlipbookComponent.SetFlipbook` (`self.EnemyFlipbook`) "/Game/04Assets/Packs/Sprites/Enemies/Zombie/FB_ZombieWalk.FB_ZombieWalk")
            (`ActorComponent.Activate` (`self.CharacterMovement`) false)
            (`self.MoveToPlayerAgain`)
            (goto _label_3 :!via `Reset`)))))
    (:`OnFail`
      (bind _asbp_first_person_character (cast `/Game/01Blueprints/BP_FirstPersonCharacter` (stale `self.ReceiveBeginPlay` _output_get) :!label _label_4))
      (set `self.CanSeePlayer?` true)
      (goto _label_2))))

(event `self.ReceiveBeginPlay`
  ;[0 0 0] Get player reference
  (bind _returnvalue (`GameplayStatics.GetActorOfClass` "/Game/01Blueprints/BP_FirstPersonCharacter.BP_FirstPersonCharacter_C"))
  (bind _output_get (set `self.PlayerRef` _returnvalue))
  (goto _label_4))

(event `self.PawnSensing.OnSeePawn`
  (params (Pawn :type "Pawn Object Reference"))
  ;[0 0 0] When see player move towards
)

(event `DamageMeleeEnemy`
  ;[0 0 0] When shot stop movement and play stun anim then after delay react movement and play moving anim
  (`PaperFlipbookComponent.SetFlipbook` (`self.EnemyFlipbook`) "/Game/04Assets/Packs/Sprites/Enemies/Zombie/FB_ZombieTakeDamage.FB_ZombieTakeDamage")
  (`ActorComponent.Deactivate` (`self.CharacterMovement`))
  (`KismetSystemLibrary.Delay` 0.2)
  (`PaperFlipbookComponent.SetFlipbook` (`self.EnemyFlipbook`) "/Game/04Assets/Packs/Sprites/Enemies/Zombie/FB_ZombieWalk.FB_ZombieWalk")
  (`ActorComponent.Activate` (`self.CharacterMovement`) false))

(event `AttackPlayer`
  ;[0 0 0] When attacking player call take damage on player
  (bind _asbp_first_person_character (cast `/Game/01Blueprints/BP_FirstPersonCharacter` (`self.PlayerRef`)))
  (`/Game/01Blueprints/BP_FirstPersonCharacter.TakeMeleeDamage` _asbp_first_person_character))

(event `KillMeleeEnemy`
  (bind _enemyflipbook (`self.EnemyFlipbook`))
  (`KismetSystemLibrary.PrintString` "kill melee enemy called")
  (`/Engine/EditorBlueprintResources/StandardMacros.DoOnce` false
    (:`Completed`
      (`KismetSystemLibrary.Delay` 0.2)
      ;[0 0 0] When kill enemy called enable is dead,  deactivate movement, deactivate capsule component, play death anim, after play dead sprite and then after delay destroy self
      (set `self.IsDead?` true)
      (`ActorComponent.Deactivate` (`self.CharacterMovement`))
      (`KismetSystemLibrary.PrintString` "movement off")
      (`GameplayStatics.PlaySound2D` "/Game/04Assets/Audio/Zombie/zombieDeath.zombieDeath" 1.0 1.0 0.0 null null)
      (`PaperFlipbookComponent.SetFlipbook` _enemyflipbook "/Game/04Assets/Packs/Sprites/Enemies/Zombie/FB_ZombieDeath.FB_ZombieDeath")
      (`KismetSystemLibrary.Delay` (`PaperFlipbookComponent.GetFlipbookLength` _enemyflipbook))
      (`KismetSystemLibrary.PrintString` "death anim played")
      (`|SpawnActorFromClass` "/Game/01Blueprints/Pickups/BP_PistolAmmoPickup.BP_PistolAmmoPickup_C" (`self.GetTransform`) "Undefined" "MultiplyWithRoot" null null)
      (`ActorComponent.K2_DestroyComponent` (`self.CapsuleComponent`))
      (`PaperFlipbookComponent.SetFlipbook` (`self.EnemyFlipbook`) "/Game/04Assets/Packs/Sprites/Enemies/Zombie/FB_ZombieDeadBody.FB_ZombieDeadBody")
      (bind _asbp_zombies_mode (cast `/Game/01Blueprints/Gamemodes/BP_ZombiesMode` (`GameplayStatics.GetGameMode`)))
      (`/Game/01Blueprints/Gamemodes/BP_ZombiesMode.ZombieKilled` _asbp_zombies_mode)
      (`KismetSystemLibrary.Delay` 4.0)
      (`self.K2_DestroyActor`)
      (`KismetSystemLibrary.PrintString` "actor destroyed"))))

(fn `UserConstructionScript`)